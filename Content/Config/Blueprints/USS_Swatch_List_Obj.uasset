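; USS_Swatch_List_Obj is an object wrapper around one USS swatch struct, holding its name, priority, material and primary and secondary colors.
; Setters edit the struct and call RefreshSwatch, with priority changes also passed to the SwatchList and refreshed only when it is valid.
; RefreshSwatch writes the struct into GroupRef's swatch array at this object's index, or appends it, then refreshes the group.
; Removal flags deletion and drops that struct entry.
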(fn SetPrimaryColor
  (params (Primary%20Color :type Text))
  (Utilities|Struct|SetmembersinUSSSwatch (Variables|Default|GetSwatch) (Utilities|String|ToString(Text) Primary%20Color))
  (CallFunction|RefreshSwatch))

(fn SetSecondaryColor
  (params (Secondary%20Color :type Text))
  (Utilities|Struct|SetmembersinUSSSwatch (Variables|Default|GetSwatch) (Utilities|String|ToString(Text) Secondary%20Color))
  (CallFunction|RefreshSwatch))

(fn SetName
  (params (Name :type Text))
  (Utilities|Struct|SetmembersinUSSSwatch (Variables|Default|GetSwatch) Name)
  (CallFunction|RefreshSwatch))

(fn SetPriority
  (params (Priority :type Integer))
  (bind _swatchlist (Variables|Default|GetSwatchList))
  (Utilities|Struct|SetmembersinUSSSwatch (Variables|Default|GetSwatch) (Math|Conversions|ToFloat(Integer) Priority))
  (Utilities|IsValid _swatchlist
    (:Is%20Valid
      (Default|UpdatePriority _swatchlist Priority)
      (CallFunction|RefreshSwatch))))

(fn SetMaterial
  (params (Material :type EUSSSwatchMaterial%20Enum :default "Default"))
  (Utilities|Struct|SetmembersinUSSSwatch (Variables|Default|GetSwatch) Material)
  (CallFunction|RefreshSwatch))

(fn InitSwatch
  (params (Swatch :type USS%20Swatch%20Structure))
  (Variables|Default|SetSwatch Swatch)
  (bind _name (Getters|GetName))
  (Class|BlueprintLoggingLibrary|LogDisplay (Utilities|String|ToString(Text) _name)))

(fn SetSwatchList
  (params (List :type USS%20Swatch%20List%20Object%20Reference))
  (Variables|Default|SetSwatchList List))

(fn SetParentList
  (params (List :type List%20View%20Object%20Reference)))

(fn GetSwatchList
  (return (Variables|Default|GetSwatchList)))

(fn GetName
  (return (Utilities|Struct|BreakUSSSwatch (Variables|Default|GetSwatch))))

(fn GetPrimaryColor
  (return (Utilities|Struct|BreakUSSSwatch (Variables|Default|GetSwatch))))

(fn GetSecondaryColor
  (return (Utilities|Struct|BreakUSSSwatch (Variables|Default|GetSwatch))))

(fn GetPriority
  (return (Math|Float|Truncate (Utilities|Struct|BreakUSSSwatch (Variables|Default|GetSwatch)))))

(fn GetMaterial
  (return (Utilities|Struct|BreakUSSSwatch (Variables|Default|GetSwatch))))

(fn GetParentList
  (return 0))

(fn SetGroupRef
  (params (Group :type USS%20Group%20List%20Obj%20Object%20Reference))
  (Variables|Default|SetGroupRef Group))

(fn ToString
  (bind _swatch (Variables|Default|GetSwatch))
  (bind (_name _priority _material _primarycolor _secondarycolor) (Utilities|Struct|BreakUSSSwatch _swatch))
  (return (Utilities|String|Append "            Swatch : " (Utilities|String|ToString(Text) _name) " 
               - Priority : " (Utilities|String|ToString(Float) _priority) " 
               - Material : " (Utilities|String|EnumtoString _material) " 
               - Primary color : " _primarycolor " 
               - Secondary color : " _secondarycolor " 
")))

(fn RemoveSwatchfromGroup
  (bind _self self)
  (bind _groupref (Variables|Default|GetGroupRef))
  (Class|BlueprintLoggingLibrary|LogDisplay "Removing Swatch")
  (Variables|USS_Swatch_List_Obj_C|SetIsMarkedAsDeleted _self true)
  (Utilities|IsValid _groupref
    (:Is%20Valid
      (Utilities|Array|RemoveIndex (Utilities|Struct|BreakUSSGroup (Variables|/UniversalSwatchSlots/Config/Blueprints/USS_Group_List_Obj.USS_Group_List_Obj_C|GetStructRef _groupref)) (Utilities|Array|FindItem (Variables|/UniversalSwatchSlots/Config/Blueprints/USS_Group_List_Obj.USS_Group_List_Obj_C|GetSwatches _groupref) _self))
      (Default|RefreshGroup (Variables|Default|GetGroupRef)))))

(fn RefreshSwatch
  (bind _self self)
  (bind _swatch (Variables|Default|GetSwatch))
  (bind _groupref (Variables|Default|GetGroupRef))
  (bind _structref (Variables|/UniversalSwatchSlots/Config/Blueprints/USS_Group_List_Obj.USS_Group_List_Obj_C|GetStructRef _groupref))
  (bind _swatches (Variables|/UniversalSwatchSlots/Config/Blueprints/USS_Group_List_Obj.USS_Group_List_Obj_C|GetSwatches _groupref))
  (bind _swatches_2 (Utilities|Struct|BreakUSSGroup _structref))
  (bind _returnvalue (Utilities|Array|FindItem _swatches _self))
  (Utilities|IsValid _groupref
    (:Is%20Valid
      (if (!= _returnvalue -1)
        (Utilities|Array|SetArrayElem _swatches_2 _returnvalue _swatch)
        (else
          (Utilities|Array|Add _swatches_2 _swatch)))
      (Default|RefreshGroup (Variables|Default|GetGroupRef)))))

(fn InitSwatchfromStruct
  (params (Swatch%20List :type USS%20Swatch%20List%20Object%20Reference) (Swatch%20ID :type Integer) (Swatch :type USS%20Swatch%20Structure))
  (Variables|Default|SetSwatchList Swatch%20List)
  (Variables|Default|SetSwatchID Swatch%20ID)
  (Variables|Default|SetSwatch Swatch))