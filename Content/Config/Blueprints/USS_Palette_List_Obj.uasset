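; USS list item object that wraps a palette struct and links it to its list widget, parent list and owner.
; Accessors edit the name, active state and primary/secondary color add/remove flags, with active state mirrored to the widget's checkbox.
; Group objects parallel the struct's group array, and refresh writes their structs back into the palette.
; Initializing from a struct sorts groups by priority and fills the widget's group list view.
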(fn SetName
  (params (Name :type Text))
  (Utilities|Struct|SetmembersinUSSPalette (Variables|Default|GetStructRef) Name))

(fn AddGroup
  (params (Group :type USS%20Group%20List%20Obj%20Object%20Reference) (At :type Integer))
  (if (< At (Utilities|Array|Length (Variables|Default|GetGroups)))
    (Utilities|Array|Insert (Variables|Default|GetGroups) Group At)
    (Utilities|Array|Insert (Utilities|Struct|BreakUSSPalette (Variables|Default|GetStructRef)) (Variables|/UniversalSwatchSlots/Config/Blueprints/USS_Group_List_Obj.USS_Group_List_Obj_C|GetStructRef Group) At)
    (else
      (Utilities|Array|Add (Variables|Default|GetGroups) Group)
      (Utilities|Array|Add (Utilities|Struct|BreakUSSPalette (Variables|Default|GetStructRef)) (Variables|/UniversalSwatchSlots/Config/Blueprints/USS_Group_List_Obj.USS_Group_List_Obj_C|GetStructRef Group))))
  (Default|SetPaletteRef Group self))

(fn InitPalette
  (params (Palette :type USS%20Palette%20Structure))
  (Variables|Default|SetStructRef Palette))

(fn SetPaletteList
  (params (List :type USS%20Palette%20List%20Object%20Reference))
  (Variables|Default|SetPaletteList List))

(fn SetParentList
  (params (List :type List%20View%20Object%20Reference))
  (Variables|Default|SetParentList List))

(fn SetIsActive
  (params (IsActive :type Boolean))
  (bind _palettelist (Variables|Default|GetPaletteList))
  (bind _is_active_box (Variables|/UniversalSwatchSlots/Config/Widgets/USS_Palette_List.USS_Palette_List_C|GetIs_Active_Box _palettelist))
  (Utilities|Struct|SetmembersinUSSPalette (Variables|Default|GetStructRef) IsActive)
  (if IsActive
    (Variables|/Script/UMG.CheckBox|SetCheckedState _is_active_box "Checked")
    (else
      (Variables|/Script/UMG.CheckBox|SetCheckedState _is_active_box "Unchecked"))))

(fn SetAddPrimaryColors
  (params (IsActive :type Boolean))
  (Utilities|Struct|SetmembersinUSSPalette (Variables|Default|GetStructRef) IsActive))

(fn SetAddSecondaryColors
  (params (IsActive :type Boolean))
  (Utilities|Struct|SetmembersinUSSPalette (Variables|Default|GetStructRef) IsActive))

(fn GetMainOwner
  (return (Variables|Default|GetMainOwner)))

(fn GetName
  (return (Utilities|Struct|BreakUSSPalette (Variables|Default|GetStructRef))))

(fn GetPaletteList
  (return (Variables|Default|GetPaletteList)))

(fn GetParentList
  (return (Variables|Default|GetParentList)))

(fn GetIsActive
  (return (.IsActive (Utilities|Struct|BreakUSSPalette (Variables|Default|GetStructRef)))))

(fn GetAddPrimaryColors
  (return (.AddPrimaryColorsToPreset (Utilities|Struct|BreakUSSPalette (Variables|Default|GetStructRef)))))

(fn GetAddSecondaryColors
  (return (Utilities|Struct|BreakUSSPalette (Variables|Default|GetStructRef))))

(fn InitPaletteGroups
  (bind _groups (Variables|Default|GetGroups))
  (bind _structref (Variables|Default|GetStructRef))
  (bind _groups_2 (Utilities|Struct|BreakUSSPalette _structref))
  (for _array_element _groups_2
    (Class|BlueprintLoggingLibrary|LogDisplay (Utilities|String|Append (Utilities|String|ToString(Text) (.Name (Utilities|Struct|BreakUSSGroup _array_element))) (Utilities|String|ToString(Integer) (Utilities|Array|Length (.Swatches (Utilities|Struct|BreakUSSGroup _array_element)))))))
  (LocalVariables|SetTmpArray _groups_2)
  (FromStruct|ResetGroups)
  (for _array_element_2 (LocalVariables|GetTmpArray)
    (Default|AddGroup (Variables|Default|GetPaletteList) false _array_element_2))
  (Class|BlueprintLoggingLibrary|LogDisplay (Utilities|String|Append "num of G : " (Utilities|String|ToString(Integer) (Utilities|Array|Length _groups))))
  (for _array_element_3 _groups
    (Class|BlueprintLoggingLibrary|LogDisplay (Utilities|String|Append (Utilities|String|ToString(Integer) (Utilities|Array|Length (.Swatches (Utilities|Struct|BreakUSSGroup (Variables|/UniversalSwatchSlots/Config/Blueprints/USS_Group_List_Obj.USS_Group_List_Obj_C|GetStructRef _array_element_3))))) (Utilities|String|ToString(Text) (.Name (Utilities|Struct|BreakUSSGroup (Variables|/UniversalSwatchSlots/Config/Blueprints/USS_Group_List_Obj.USS_Group_List_Obj_C|GetStructRef _array_element_3))))))))

(fn SetMainOwner
  (params (Owner :type USS%20Custom%20Config%20Widget%20Object%20Reference))
  (Variables|Default|SetMainOwner Owner))

(fn ToString
  (bind _groups (Variables|Default|GetGroups))
  (bind _structref (Variables|Default|GetStructRef))
  (bind (_palettename _isactive _addprimarycolorstopreset _addsecondarycolorstopreset) (Utilities|Struct|BreakUSSPalette _structref))
  (for _array_element _groups
    (bind _string (Default|ToString _array_element))
    (LocalVariables|SetGroupStr (Utilities|String|Append (LocalVariables|GetGroupStr) _string)))
  (return (Utilities|String|Append " 
Palette : " (Utilities|String|ToString(Text) _palettename) " 
   - Active : " (Utilities|String|ToString(Boolean) _isactive) " 
   - Add primary colors  : " (Utilities|String|ToString(Boolean) _addprimarycolorstopreset) " 
   - Add secondary colors : " (Utilities|String|ToString(Boolean) _addsecondarycolorstopreset) " 
   - Number of groups : " (Utilities|String|ToString(Integer) (Utilities|Array|Length _groups)) " 
" (LocalVariables|GetGroupStr))))

(fn ResetGroups
  (bind _groups (Variables|Default|GetGroups))
  (bind _returnvalue (Utilities|Array|Length _groups))
  (Class|BlueprintLoggingLibrary|LogDisplay (Utilities|String|Append "azdz" (Utilities|String|ToString(Integer) _returnvalue)))
  (if (== _returnvalue 0)
    _
    (else
      (Utilities|Array|Clear _groups)))
  (Utilities|Array|Clear (Utilities|Struct|BreakUSSPalette (Variables|Default|GetStructRef))))

(fn RefreshPalette
  (Default|ExpandList (Variables|Default|GetPaletteList) true)
  (for _array_element (Variables|Default|GetGroups)
    (Default|RefreshGroup _array_element)
    (Utilities|Array|Add (LocalVariables|GetUpdatedGroups) (Variables|/UniversalSwatchSlots/Config/Blueprints/USS_Group_List_Obj.USS_Group_List_Obj_C|GetStructRef _array_element)))
  (Utilities|Struct|SetmembersinUSSPalette (Variables|Default|GetStructRef) (LocalVariables|GetUpdatedGroups)))

(fn GetRemovePrimaryColors
  (return (Utilities|Struct|BreakUSSPalette (Variables|Default|GetStructRef))))

(fn GetRemoveSecondaryColors
  (return (Utilities|Struct|BreakUSSPalette (Variables|Default|GetStructRef))))

(fn SetRemovePrimaryColors
  (params (IsActive :type Boolean))
  (Utilities|Struct|SetmembersinUSSPalette (Variables|Default|GetStructRef) IsActive))

(fn SetRemoveSecondaryColors
  (params (IsActive :type Boolean))
  (Utilities|Struct|SetmembersinUSSPalette (Variables|Default|GetStructRef) IsActive))

(fn InitPaletteListfromStruct
  (params (Palette%20List :type USS%20Palette%20List%20Object%20Reference) (Struct :type USS%20Palette%20Structure))
  (bind _self self)
  (Variables|Default|SetPaletteList Palette%20List)
  (bind _output_get (Variables|Default|SetStructRef Struct))
  (|ArraySort (Utilities|Struct|BreakUSSPalette _output_get))
  (for (_array_element _array_index) (Utilities|Struct|BreakUSSPalette _output_get)
    (Development|PrintString _self (Utilities|String|Append "Add group " (Utilities|String|ToString(Text) (.Name (Utilities|Struct|BreakUSSGroup _array_element))) " to palette. Num of swatches : " (Utilities|String|ToString(Integer) (Utilities|Array|Length (.Swatches (Utilities|Struct|BreakUSSGroup _array_element))))))
    (bind _returnvalue (Game|ConstructObjectfromClass "/UniversalSwatchSlots/Config/Widgets/USS_Group_List.USS_Group_List_C"))
    (Development|PrintString _self (Utilities|String|Append "Group Ref : " (Utilities|GetDisplayName _returnvalue)))
    (Default|InitGroupListfromPalette _returnvalue self _array_element _array_index)
    (Class|ListView|AddItem (Getters|GetPaletteGroupListView) _returnvalue)
    (Development|PrintString _self (Utilities|String|ToString(Integer) (Utilities|Array|Length (Class|ListView|GetListItems (Getters|GetPaletteGroupListView)))))))

(fn GetPaletteGroupListView
  (bind _palettelist (Variables|Default|GetPaletteList))
  (bind _list_view (Default|GetPaletteGroupListView _palettelist))
  (Development|PrintString 0 (Utilities|GetDisplayName _list_view))
  (return _list_view))

(fn USSPaletteListObjUSSGroupStructureComparator
  (params (A :type USS%20Group%20Structure) (B :type USS%20Group%20Structure))
  (return (< (.Priority (Utilities|Struct|BreakUSSGroup A)) (.Priority (Utilities|Struct|BreakUSSGroup B)))))