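; List data object for one USS swatch, holding its name, priority, material and primary and secondary colors as strings.
; Setters edit the swatch struct, then RefreshSwatch writes it into the parent group's array by list-view index (or appends it) and refreshes the group.
; Priority is stored minus one and only triggers a refresh when the entry widget is valid.
; Add, remove and dirty-marking delegate to the group data entry.
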(fn SetPrimaryColor
  (params (Primary%20Color :type Text))
  (Utilities|Struct|SetmembersinUSSSwatch (Variables|Default|GetSwatch) (Utilities|String|ToString(Text) Primary%20Color))
  (CallFunction|RefreshSwatch))

(fn SetSecondaryColor
  (params (Secondary%20Color :type Text))
  (Utilities|Struct|SetmembersinUSSSwatch (Variables|Default|GetSwatch) (Utilities|String|ToString(Text) Secondary%20Color))
  (CallFunction|RefreshSwatch))

(fn SetName
  (params (Name :type Text))
  (Utilities|Struct|SetmembersinUSSSwatch (Variables|Default|GetSwatch) Name)
  (CallFunction|RefreshSwatch))

(fn SetPriority
  (params (Priority :type Integer))
  (bind _swatchlistentry (Variables|Default|GetSwatchListEntry))
  (Utilities|Struct|SetmembersinUSSSwatch (Variables|Default|GetSwatch) (- Priority 1))
  (Utilities|IsValid _swatchlistentry
    (:Is%20Valid
      (Default|UpdatePriority _swatchlistentry Priority)
      (CallFunction|RefreshSwatch))))

(fn SetMaterial
  (params (Material :type EUSSSwatchMaterial%20Enum :default "Default"))
  (Utilities|Struct|SetmembersinUSSSwatch (Variables|Default|GetSwatch) Material)
  (CallFunction|RefreshSwatch))

(fn SetSwatchList
  (params (List :type %20Object%20Reference)))

(fn SetParentList
  (params (List :type List%20View%20Object%20Reference))
  (Variables|Default|SetParentList List))

(fn GetSwatchListEntry
  (return (Variables|Default|GetSwatchListEntry)))

(fn GetParentList
  (bind _parentlist (Variables|Default|GetParentList))
  (Utilities|PrintObjectRef _parentlist
    (:Out
      (return _parentlist))))

(fn ToString
  (bind _swatch (Variables|Default|GetSwatch))
  (bind (_name _priority _material _primarycolor _secondarycolor) (Utilities|Struct|BreakUSSSwatch _swatch))
  (return (Utilities|String|Append "            Swatch : " (Utilities|String|ToString(Text) _name) " 
               - Priority : " (Utilities|String|ToString(Integer) _priority) " 
               - Material : " (Utilities|String|EnumtoString _material) " 
               - Primary color : " _primarycolor " 
               - Secondary color : " _secondarycolor " 
")))

(fn RemoveSwatchfromGroup
  (Default|RemoveSwatchfromGroup (Variables|Default|GetGroupListDataEntryRef) self)
  (Variables|Default|SetSwatch "")
  (Variables|Default|SetGroupListDataEntryRef 0)
  (Variables|Default|SetSwatchListEntry 0))

(fn RefreshSwatch
  (bind _self self)
  (bind _grouplistdataentryref (Variables|Default|GetGroupListDataEntryRef))
  (bind _swatch (Variables|Default|GetSwatch))
  (bind _swatch_list_view (Default|GetGroupSwatchListView _grouplistdataentryref))
  (bind _group (Variables|/UniversalSwatchSlots/Config/Blueprints/USS_Group_List_Data_Entry.USS_Group_List_Data_Entry_C|GetGroup _grouplistdataentryref))
  (bind _swatches (Utilities|Struct|BreakUSSGroup _group))
  (bind _returnvalue (Class|ListView|GetListItems _swatch_list_view))
  (bind _returnvalue_2 (Utilities|Array|FindItem _returnvalue _self))
  (bind _output (Utilities|Array|Get(acopy) _swatches _returnvalue_2))
  (bind (_name _priority _material _primarycolor _secondarycolor) (Utilities|Struct|BreakUSSSwatch _output))
  (if (!= _returnvalue_2 -1)
    (Utilities|Array|SetArrayElem _swatches _returnvalue_2 _swatch)
    (else
      (Utilities|Array|Add _swatches _swatch)))
  (Development|PrintString self (Utilities|String|Append (Utilities|String|ToString(Text) _name) ", " (Utilities|String|ToString(Integer) _priority) ", " (Utilities|String|EnumtoString _material) ", " _primarycolor ", " _secondarycolor))
  (Default|RefreshGroup (Variables|Default|GetGroupListDataEntryRef)))

(fn SetGroupListDataEntry
  (params (Group%20Data%20Entry :type USS%20Group%20List%20Data%20Entry%20Object%20Reference))
  (Variables|Default|SetGroupListDataEntryRef Group%20Data%20Entry))

(fn SetSwatchStructure
  (params (Swatch :type USS%20Swatch%20Structure%20%28by%20ref%29))
  (Variables|Default|SetSwatch Swatch))

(fn SetSwatchListEntry
  (params (List :type USS%20Swatch%20List%20Entry%20Object%20Reference))
  (Variables|Default|SetSwatchListEntry List))

(fn AddNewSwatchtoGroup
  (Default|AddNewSwatchtoGroup (Variables|Default|GetGroupListDataEntryRef) self))

(fn MarkSwatchasDirty
  (Default|MarkGroupasDirty (Variables|Default|GetGroupListDataEntryRef)))