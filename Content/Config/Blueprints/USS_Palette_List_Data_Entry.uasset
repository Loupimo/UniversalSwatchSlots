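; List-view data object for one palette in the USS config UI, wrapping the palette struct with accessors for name, active state and primary/secondary color add/remove flags.
; It builds group data entries sorted by priority for the entry widget's nested list, updating the struct and renumbering priorities on insertion or removal.
; Name checks, palette creation, removal and dirty marking go to the config owner, with the old name kept for renames.
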(fn SetName
  (params (Name :type Text))
  (bind _palette (Variables|Default|GetPalette))
  (Variables|Default|SetOldName (Utilities|Struct|BreakUSSPalette _palette))
  (Utilities|Struct|SetmembersinUSSPalette _palette Name))

(fn SetIsActive
  (params (IsActive :type Boolean))
  (bind _palettelistentry (Variables|Default|GetPaletteListEntry))
  (bind _is_active_box (Variables|/UniversalSwatchSlots/Config/Widgets/USS_Palette_List_Entry.USS_Palette_List_Entry_C|GetIs_Active_Box _palettelistentry))
  (Utilities|Struct|SetmembersinUSSPalette (Variables|Default|GetPalette) IsActive)
  (if IsActive
    (Variables|/Script/UMG.CheckBox|SetCheckedState _is_active_box "Checked")
    (else
      (Variables|/Script/UMG.CheckBox|SetCheckedState _is_active_box "Unchecked"))))

(fn SetAddPrimaryColors
  (params (IsActive :type Boolean))
  (Utilities|Struct|SetmembersinUSSPalette (Variables|Default|GetPalette) IsActive))

(fn SetAddSecondaryColors
  (params (IsActive :type Boolean))
  (Utilities|Struct|SetmembersinUSSPalette (Variables|Default|GetPalette) IsActive))

(fn GetMainOwner
  (return (Variables|Default|GetConfigOwner)))

(fn GetName
  (return (Utilities|Struct|BreakUSSPalette (Variables|Default|GetPalette))))

(fn GetPaletteList
  (return (Variables|Default|GetPaletteListEntry)))

(fn GetParentList
  (return (Variables|Default|GetParentList)))

(fn GetIsActive
  (return (Utilities|Struct|BreakUSSPalette (Variables|Default|GetPalette))))

(fn GetAddPrimaryColors
  (return (Utilities|Struct|BreakUSSPalette (Variables|Default|GetPalette))))

(fn GetAddSecondaryColors
  (return (Utilities|Struct|BreakUSSPalette (Variables|Default|GetPalette))))

(fn InitPaletteGroups
  (bind _palette (Variables|Default|GetPalette))
  (bind _groups (Utilities|Struct|BreakUSSPalette _palette))
  (Development|PrintString self "Init groups")
  (|ArraySort _groups)
  (for _array_element _groups
    ;[1 1 1] Set up the Group list data entry
    (bind _create_group_entry_data (CallFunction|CreateGroupListEntryDatafromStruct _array_element))
    ;[1 1 1] Add the data list entry and triggers the Group List Entry Object Item Set Event
    (Class|ListView|AddItem (Default|GetGroupListView (Variables|Default|GetPaletteListEntry)) _create_group_entry_data)))

(fn SetMainOwner
  (params (Owner :type USS%20Custom%20Config%20Widget%20Object%20Reference))
  (Variables|Default|SetConfigOwner Owner))

(fn ToString
  (bind _palette (Variables|Default|GetPalette))
  (bind (_palettename _isactive _addprimarycolorstopreset _addsecondarycolorstopreset _removeprimarycolorstopreset _removesecondarycolorstopreset _groups) (Utilities|Struct|BreakUSSPalette _palette))
  (for _array_element (Variables|Default|GetGroupDataEntries)
    (bind _string (Default|ToString _array_element))
    (LocalVariables|SetGroupStr (Utilities|String|Append (LocalVariables|GetGroupStr) _string)))
  (return (Utilities|String|Append " 
Palette : " (Utilities|String|ToString(Text) _palettename) " 
   - Active : " (Utilities|String|ToString(Boolean) _isactive) " 
   - Add primary colors  : " (Utilities|String|ToString(Boolean) _addprimarycolorstopreset) " 
   - Add secondary colors : " (Utilities|String|ToString(Boolean) _addsecondarycolorstopreset) " 
   - Remove primary colors : " (Utilities|String|ToString(Boolean) _removeprimarycolorstopreset) " 
   - Remove secondary colors : " (Utilities|String|ToString(Boolean) _removesecondarycolorstopreset) " 
   - Number of groups : " (Utilities|String|ToString(Integer) (Utilities|Array|Length _groups)) " 
" (LocalVariables|GetGroupStr))))

(fn ResetGroups)

(fn GetRemovePrimaryColors
  (return (Utilities|Struct|BreakUSSPalette (Variables|Default|GetPalette))))

(fn GetRemoveSecondaryColors
  (return (Utilities|Struct|BreakUSSPalette (Variables|Default|GetPalette))))

(fn SetRemovePrimaryColors
  (params (IsActive :type Boolean))
  (Utilities|Struct|SetmembersinUSSPalette (Variables|Default|GetPalette) IsActive))

(fn SetRemoveSecondaryColors
  (params (IsActive :type Boolean))
  (Utilities|Struct|SetmembersinUSSPalette (Variables|Default|GetPalette) IsActive))

(fn GetPaletteGroupListView
  (return (Default|GetGroupListView (Variables|Default|GetPaletteListEntry))))

(fn USSPaletteListObjUSSGroupStructureComparator
  (params (A :type USS%20Group%20Structure) (B :type USS%20Group%20Structure))
  (return (< (.Priority (Utilities|Struct|BreakUSSGroup A)) (Math|Conversions|ToFloat(Integer) (.Priority (Utilities|Struct|BreakUSSGroup B))))))

(fn SetPaletteListEntry
  (params (Palette%20List :type USS%20Palette%20List%20Entry%20Object%20Reference))
  (Variables|Default|SetPaletteListEntry Palette%20List))

(fn SetParentList
  (params (Parent%20List :type List%20View%20Object%20Reference))
  (Variables|Default|SetParentList Parent%20List))

(fn SetPaletteStructure
  (params (Palette :type USS%20Palette%20Structure%20%28by%20ref%29))
  (bind _output_get (Variables|Default|SetPalette Palette))
  (Variables|Default|SetOldName (Utilities|Struct|BreakUSSPalette _output_get)))

(fn AddNewGrouptoPalette
  (params (Group%20Entry%20Data :type USS%20Group%20List%20Data%20Entry%20Object%20Reference))
  (Development|PrintString self "Adding new group to palette")
  (bind (_inserted_id _new_group_entry_data) (Default|AddNewGroup (Getters|GetPaletteList) Group%20Entry%20Data))
  (CallFunction|InsertGrouptoPalette _inserted_id _new_group_entry_data)
  (CallFunction|RefreshPaletteGroupList))

(fn CreateGroupListEntryDatafromStruct
  (params (Group :type USS%20Group%20Structure%20%28by%20ref%29))
  ;[1 1 1] Set up the Group list data entry
  (bind _returnvalue (Game|ConstructObjectfromClass "/UniversalSwatchSlots/Config/Blueprints/USS_Group_List_Data_Entry.USS_Group_List_Data_Entry_C"))
  (Default|SetPaletteListDataEntry _returnvalue self)
  (Default|SetGroupStructure _returnvalue Group)
  (Default|SetParentList _returnvalue (Default|GetGroupListView (Variables|Default|GetPaletteListEntry)))
  (return _returnvalue))

(fn InsertGrouptoPalette
  (params (Insert%20ID :type Integer) (Group%20Entry%20Data :type USS%20Group%20List%20Data%20Entry%20Object%20Reference))
  (bind _palette (Variables|Default|GetPalette))
  (bind _groups (Utilities|Struct|BreakUSSPalette _palette))
  (Utilities|Array|Insert _groups (Variables|/UniversalSwatchSlots/Config/Blueprints/USS_Group_List_Data_Entry.USS_Group_List_Data_Entry_C|GetGroup Group%20Entry%20Data) Insert%20ID)
  (Development|PrintString self (Utilities|String|Append "Group in the palette structure : " (Utilities|String|ToString(Integer) (Utilities|Array|Length _groups)))))

(fn RefreshPaletteGroupList
  (for (_array_element _array_index) (Class|ListView|GetListItems (Getters|GetPaletteGroupListView))
    (bind _asuss_group_list_data_entry (Utilities|Casting|CastToUSS_Group_List_Data_Entry _array_element))
    (Default|SetPriority _asuss_group_list_data_entry (+ _array_index 1))))

(fn RemoveGroupfromPalette
  (params (Group%20Entry%20Data :type USS%20Group%20List%20Data%20Entry%20Object%20Reference))
  (bind _group_list_view (Getters|GetPaletteGroupListView))
  (bind _output_get (LocalVariables|SetRemove%20ID (Utilities|Array|FindItem (Class|ListView|GetListItems _group_list_view) Group%20Entry%20Data)))
  (if (!= _output_get -1)
    (Class|ListView|RemoveItem _group_list_view Group%20Entry%20Data)
    (Utilities|Array|RemoveIndex (Utilities|Struct|BreakUSSPalette (Variables|Default|GetPalette)) (LocalVariables|GetRemove%20ID))
    (CallFunction|RefreshPaletteGroupList)))

(fn RemovePalette
  (Default|RemovePalette (Variables|Default|GetConfigOwner) self)
  (Variables|Default|SetPalette "")
  (Variables|Default|SetConfigOwner 0)
  (Variables|Default|SetPaletteListEntry 0))

(fn MarkPaletteasDirty
  (Default|MarkPaletteasDirty (Variables|Default|GetConfigOwner) self (Variables|Default|GetOldName)))

(fn AddNewPalette
  (Default|AddPalette (Variables|Default|GetConfigOwner)))

(fn CheckName
  (params (New%20Name :type Text))
  (bind _is_unique (Default|CheckPaletteName (Variables|Default|GetConfigOwner) New%20Name self))
  (return _is_unique))