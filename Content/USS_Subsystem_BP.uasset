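; Subsystem actor that registers new swatch colours with the Buildable Subsystem and opts into saving.
; For each swatch descriptor whose ID is not a valid index in the colour slot array, it pads the array with black slots up to that ID.
; It then writes the descriptor's primary and secondary colours into that slot by reference, leaving already existing slots untouched.
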(event EventBeginPlay)

(fn ConstructionScript)

(fn ShouldSave
  (return true))

(fn AddNewSwatchesColorstoBuildableSubsystem
  (params (SwatchDescriptors :type Array%20of%20USS%20Swatch%20Desc%20Object%20References))
  (bind _returnvalue (Class|FGBuildableSubsystem|Get))
  (bind _mcolorslots_data (Variables|/Script/FactoryGame.FGBuildableSubsystem|GetmColorSlots_Data _returnvalue))
  (for _array_element SwatchDescriptors
    (if (not (Utilities|Array|IsValidIndex _mcolorslots_data (Variables|/Script/FactoryGame.FGFactoryCustomizationDescriptor|GetID _array_element)))
      (for _index (range (Utilities|Array|Length _mcolorslots_data) (Variables|/Script/FactoryGame.FGFactoryCustomizationDescriptor|GetID _array_element))
        (Utilities|Array|Add _mcolorslots_data (Class|FGBlueprintFunctionLibrary|MakeCustomizationColorSlot :Finish "/Game/FactoryGame/Buildable/-Shared/Customization/PaintFinishes/PaintFinishDesc_Default.PaintFinishDesc_Default_C")))
      (|SetBy-RefVar (Utilities|Array|Get(acopy) _mcolorslots_data (Variables|/Script/FactoryGame.FGFactoryCustomizationDescriptor|GetID _array_element)) (Class|FGBlueprintFunctionLibrary|MakeCustomizationColorSlot (Variables|/Script/UniversalSwatchSlots.USSSwatchDesc|GetPrimaryColour _array_element) (Variables|/Script/UniversalSwatchSlots.USSSwatchDesc|GetSecondaryColour _array_element) "/Game/FactoryGame/Buildable/-Shared/Customization/PaintFinishes/PaintFinishDesc_Default.PaintFinishDesc_Default_C")))))